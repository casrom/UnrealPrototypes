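; BP_PowerColumn is a power column that animates between two relative locations, carrying its caps and two power redirectors.
; MoveCylinderEvent plays a timeline that lerps the root, while the direction flag picks which cap moves and weights the redirectors' offsets unevenly.
; The same alpha spins the redirector meshes one full yaw turn in opposite directions from rotations cached at the start.
; When the timeline finishes, it registers the energy discs.
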(event `self.MoveCylinderEvent`
  (params (BeginLocation :type "Vector Structure") (EndLocation :type "Vector Structure") (IsUp :type Boolean))
  (bind _redirectordownrotation (`self.RedirectorDownRotation`))
  (bind _redirectoruprotation (`self.RedirectorUpRotation`))
  (bind _staticvisualmesh (`PowerRedirector.StaticVisualMesh` (`self.PowerRedirectorUp`)))
  (bind _staticvisualmesh_2 (`PowerRedirector.StaticVisualMesh` (`self.PowerRedirectorDown`)))
  (set `self.RedirectorDownRotation` (`SceneComponent.RelativeRotation` _staticvisualmesh_2))
  (set `self.RedirectorUpRotation` (`SceneComponent.RelativeRotation` _staticvisualmesh))
  (bind (_direction _alpha) (`Timeline|MoveCylinder` :!via `PlayFromStart`)
    (:`Update`
      (`SceneComponent.K2_SetRelativeRotation` _staticvisualmesh (`KismetMathLibrary.RLerp` _redirectoruprotation (`KismetMathLibrary.MakeRotator` (.roll _redirectoruprotation) (.pitch _redirectoruprotation) (+ (.yaw _redirectoruprotation) 360.0)) _alpha) false false)
      (`SceneComponent.K2_SetRelativeRotation` _staticvisualmesh_2 (`KismetMathLibrary.RLerp` _redirectordownrotation (`KismetMathLibrary.MakeRotator` (.roll _redirectordownrotation) (.pitch _redirectordownrotation) (+ (.yaw _redirectordownrotation) -360.0)) _alpha) false false)
      (bind _returnvalue (`KismetMathLibrary.VLerp` BeginLocation EndLocation _alpha))
      (`SceneComponent.K2_SetRelativeLocation` (`self.Root`) _returnvalue false false)
      (if IsUp
        (bind _returnvalue_2 (* _returnvalue 1.0))
        (`SceneComponent.K2_SetRelativeLocation` (`self.CapTop`) _returnvalue_2 false false)
        (bind _returnvalue_3 (* _returnvalue 0.8))
        (`self.K2_SetActorRelativeLocation` (`self.PowerRedirectorUp`) _returnvalue_3 false false)
        (bind _returnvalue_4 (* _returnvalue 0.2))
        (`self.K2_SetActorRelativeLocation` (`self.PowerRedirectorDown`) _returnvalue_4 false false)
        (else
          (`SceneComponent.K2_SetRelativeLocation` (`self.CapBottom`) _returnvalue_2 false false)
          (`self.K2_SetActorRelativeLocation` (`self.PowerRedirectorDown`) _returnvalue_3 false false)
          (`self.K2_SetActorRelativeLocation` (`self.PowerRedirectorUp`) _returnvalue_4 false false))))
    (:`Finished`
      (`self.RegisterEnergyDiscs`))))

(fn `UserConstructionScript`)